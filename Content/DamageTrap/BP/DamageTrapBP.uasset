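; DamageTrapBP is a trap that damages the FirstPersonCharacter when it enters the DamageCollision volume.
; Each hit applies Damage, then sets a Resting flag for RestTime, during which new overlaps are ignored.
; After the rest, it loops back to damage the same character again if it still overlaps the volume.
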(event `self.damageCollision.OnComponentBeginOverlap`
  (params (OverlappedComponent :type "PrimitiveComponent Object Reference") (OtherActor :type "Actor Object Reference") (OtherComp :type "PrimitiveComponent Object Reference") (OtherBodyIndex :type Integer) (bFromSweep :type Boolean) (SweepResult :type "HitResult Structure (by ref)"))
  (if (not (`self.Resting`))
    (bind _asfirst_person_character (cast `/Game/FirstPersonBP/Blueprints/FirstPersonCharacter` OtherActor))
    (`GameplayStatics.ApplyDamage` _asfirst_person_character (`self.Damage`) :!label _label)
    (set `self.Resting` true)
    (`KismetSystemLibrary.Delay` (`self.RestTime`))
    (set `self.Resting` false)
    (if (`PrimitiveComponent.IsOverlappingActor` (`self.damageCollision`) _asfirst_person_character)
      (goto _label))))

(fn `UserConstructionScript`)